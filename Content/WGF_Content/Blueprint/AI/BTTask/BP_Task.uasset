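; Behavior tree task that sends a BP_AIController to the location stored in the Destination blackboard key.
; On execute it prints the destination, issues an AI MoveTo, sets Intialise and finishes successfully at once, without waiting for the move to end.
; Move completion and request failure only print debug strings, and the IncreaseIndex and AccelSwitch calls are left unconnected.
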(event EventReceiveExecute
  (params (OwnerActor :type Actor%20Object%20Reference))
  (bind _destination (Variables|Default|GetDestination))
  (bind _returnvalue (Class|BTFunctionLibrary|GetBlackboardValueasVector _destination))
  (bind _asbp_aicontroller (Utilities|Casting|CastToBP_AIController OwnerActor))
  (Development|PrintString (Utilities|String|ToString(Vector) _returnvalue))
  (AI|AIMoveTo _asbp_aicontroller _returnvalue 0 -1.0 "Default" "Default" true true
    (:then
      (Variables|Default|SetIntialise true)
      (AI|BehaviorTree|FinishExecute true))
    (:OnRequestFailed
      (Development|PrintString "Fail"))
    (:OnMoveFinished
      (Development|PrintString "Suc"))))
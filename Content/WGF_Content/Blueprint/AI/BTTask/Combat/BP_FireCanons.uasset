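; Behavior tree task that makes an AI-controlled ship fire a broadside of cannons, intended to target the player.
; It gets the pawn from the AI controller and instantly yaws its ship mesh a quarter turn, zeroing pitch and roll.
; The LeftRight flag selects the left or right cannons, though the rotation is the same for both, and the task then finishes successfully.
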(event EventReceiveExecute
  (params (OwnerActor :type Actor%20Object%20Reference))
  (bind _asbp_aicontroller (Utilities|Casting|CastToBP_AIController OwnerActor))
  (bind _asbp_ship_defualt (Utilities|Casting|CastToBP_ShipDefualt (Pawn|GetControlledPawn _asbp_aicontroller)))
  ;[1 1 1] turn towards the player so the cannons on the right can fire at the player
  (Transformation|SetWorldRotation (Variables|/Game/WGF_Content/Blueprint/Ship/BP_ShipDefualt.BP_ShipDefualt_C|GetShipMesh _asbp_ship_defualt) (Math|Rotator|MakeRotator 0.0 0.0 (+ (.yaw (Transformation|GetWorldRotation (Variables|/Game/WGF_Content/Blueprint/Ship/BP_ShipDefualt.BP_ShipDefualt_C|GetShipMesh _asbp_ship_defualt))) -9e+01)) false false)
  (if (Variables|Default|GetLeftRight?)
    (Default|FireLeftCannons _asbp_ship_defualt)
    (else
      (Default|FireRightCannons _asbp_ship_defualt)))
  (AI|BehaviorTree|FinishExecute true))
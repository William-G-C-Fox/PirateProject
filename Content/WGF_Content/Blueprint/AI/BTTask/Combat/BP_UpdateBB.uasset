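; Behavior Tree task that refreshes an AI ship's combat blackboard.
; On execute, it casts the owner to BP_AIController and writes the controlled BP_ShipDefualt's Health and InCombat to blackboard keys.
; It then casts that ship's Player reference to BP_ShipPlayer, writes the player's Notority and finishes successfully.
; A failed cast stops execution without calling FinishExecute.
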(event EventReceiveExecute
  (params (OwnerActor :type Actor%20Object%20Reference))
  ;[1 1 1] Updates all the player information into the black board
  (bind _asbp_aicontroller (Utilities|Casting|CastToBP_AIController OwnerActor))
  (bind _asbp_ship_defualt (Utilities|Casting|CastToBP_ShipDefualt (Pawn|GetControlledPawn _asbp_aicontroller)))
  (Class|BTFunctionLibrary|SetBlackboardValueasInt (Variables|Default|GetHealth) (Variables|/Game/WGF_Content/Blueprint/Ship/BP_ShipDefualt.BP_ShipDefualt_C|GetHealth _asbp_ship_defualt))
  (Class|BTFunctionLibrary|SetBlackboardValueasBool (Variables|Default|GetInCombat) (Variables|/Game/WGF_Content/Blueprint/Ship/BP_ShipDefualt.BP_ShipDefualt_C|GetInCombat? _asbp_ship_defualt))
  (bind _asbp_ship_player (Utilities|Casting|CastToBP_ShipPlayer (Variables|/Game/WGF_Content/Blueprint/Ship/BP_ShipDefualt.BP_ShipDefualt_C|GetPlayer _asbp_ship_defualt)))
  (Class|BTFunctionLibrary|SetBlackboardValueasInt (Variables|Default|GetNotority) (Variables|/Game/WGF_Content/Blueprint/Ship/BP_ShipPlayer.BP_ShipPlayer_C|GetNotority _asbp_ship_player))
  (AI|BehaviorTree|FinishExecute true))
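; Behavior tree task for the Hunter AI that targets the player's position and checks how close the ship is to it.
; It gets the controlled ship from the AI controller and writes the location of that ship's stored Player reference into the destination blackboard key.
; It then fails if the player is beyond a fixed distance and succeeds otherwise, with the destination updated in both cases.
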(event EventReceiveExecute
  (params (OwnerActor :type Actor%20Object%20Reference))
  (bind _asbp_aicontroller (Utilities|Casting|CastToBP_AIController OwnerActor))
  (bind _asbp_ship_defualt (Utilities|Casting|CastToBP_ShipDefualt (Pawn|GetControlledPawn _asbp_aicontroller)))
  (AI|BehaviorTree|SetBlackboardValueasVector (Variables|Default|GetDestitnation) (.location (Transformation|GetActorTransform (Variables|/Game/WGF_Content/Blueprint/Ship/BP_ShipDefualt.BP_ShipDefualt_C|GetPlayer _asbp_ship_defualt))))
  (if (> (Math|Vector|Distance(Vector) (.location (Transformation|GetActorTransform (Variables|/Game/WGF_Content/Blueprint/Ship/BP_ShipDefualt.BP_ShipDefualt_C|GetPlayer _asbp_ship_defualt))) (.location (Transformation|GetActorTransform _asbp_ship_defualt))) 1.5e+03)
    (AI|BehaviorTree|FinishExecute false)
    (else
      (AI|BehaviorTree|FinishExecute true))))
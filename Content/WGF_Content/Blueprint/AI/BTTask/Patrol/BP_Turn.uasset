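; BP_Turn is a patrol behavior tree task that tells an AI-controlled ship to turn toward a blackboard direction.
; On execute, it casts the owner to an AIController and its pawn to BP_ShipDefualt, then passes the Direction vector to the ship's AITurn, printing it for debugging.
; The task finishes successfully right after the call.
; A turn-sequence counter and a look-at rotation calculation remain as unused leftovers.
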(event EventReceiveExecute
  (params (OwnerActor :type Actor%20Object%20Reference))
  (CallFunction|Turn OwnerActor)
  (AI|BehaviorTree|FinishExecute true))

(fn Turn
  (params (Actor :type Actor%20Object%20Reference))
  (bind _direction (Variables|Default|GetDirection))
  (bind _returnvalue (Class|BTFunctionLibrary|GetBlackboardValueasVector _direction))
  (bind _asaicontroller (Utilities|Casting|CastToAIController Actor))
  (bind _asbp_ship_defualt (Utilities|Casting|CastToBP_ShipDefualt (Pawn|GetControlledPawn _asaicontroller)))
  (Development|PrintString (Utilities|String|ToString(Vector) _returnvalue))
  (Default|AITurn _asbp_ship_defualt _returnvalue))
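; BP_AudioPlayer is an actor that plays music tracks from a list.
; On BeginPlay, Intial checks the Infinite value and, in its Infinite case, stops playback and starts a random track from the first four.
; PlayAudio assigns the indexed sound to the MusicPlayer component and plays it from the start, while StopAudio halts it.
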(event EventBeginPlay
  (CallFunction|Intial))

(event Collision|EventActorBeginOverlap
  (params (OtherActor :type Actor%20Object%20Reference)))

(event EventTick
  (params (DeltaSeconds :type Float%20%28single-precision%29)))

(fn ConstructionScript)

(fn PlayAudio
  (params (TrackNum :type Integer))
  (Audio|Components|Audio|SetSound (Variables|Default|GetMusicPlayer) (Utilities|Array|Get(acopy) (Variables|Default|GetMusicList) TrackNum))
  (Audio|Components|Audio|Play (Variables|Default|GetMusicPlayer) 0.0))

(fn StopAudio
  (Audio|Components|Audio|Stop (Variables|Default|GetMusicPlayer)))

(fn Intial
  (switch Utilities|FlowControl|Switch|SwitchonENiagara_InfiniteLoopDuration "NewEnumerator1"
    (:NewEnumerator1
      (CallFunction|StopAudio)
      (CallFunction|PlayAudio (Math|Random|RandomInteger 4)))))
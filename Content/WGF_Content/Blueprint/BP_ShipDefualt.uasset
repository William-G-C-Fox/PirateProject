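; Player-controlled ship pawn that sails with a stepped throttle and fires cannon broadsides from either side.
; Forward/back inputs step an acceleration index, mapped to a scale that drives movement along the actor's right vector each tick.
; Steering yaws the ship mesh directly; TurnRate switches on a constant, so its offset stays zero.
; Mouse buttons spawn three cannonballs per side behind timer cooldowns, and TakeDamage destroys the ship at exactly zero health.
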(event EventBeginPlay)

(event Collision|EventActorBeginOverlap
  (params (OtherActor :type Actor%20Object%20Reference)))

(event EventTick
  (params (DeltaSeconds :type Float%20%28single-precision%29))
  (Pawn|Input|AddMovementInput (Transformation|GetActorRightVector) (Variables|Default|GetAccelarationScale) false))

(event Input|ActionEvents|InputActionMoveForward
  (params (Key :type Key%20Structure))
  (:Pressed
    (CallFunction|IncreaseIndex)
    (CallFunction|AccelSwitch)))

(event Input|ActionEvents|InputActionMoveBack
  (params (Key :type Key%20Structure))
  (:Pressed
    (CallFunction|DecreaseIndex)
    (CallFunction|AccelSwitch)))

(event Input|AxisEvents|InputAxisMoveRight
  (params (AxisValue :type Float%20%28single-precision%29))
  (CallFunction|Turning AxisValue))

(event Input|MouseEvents|LeftMouseButton
  (params (Key :type Key%20Structure))
  (:Pressed
    (CallFunction|FireLeftCannons)))

(event Input|MouseEvents|RightMouseButton
  (params (Key :type Key%20Structure))
  (:Pressed
    (CallFunction|FireRightCannons)))

(fn ConstructionScript)

(fn TakeDamage
  (params (Damage :type Integer))
  (bind _output_get (Variables|Default|SetHealth (- (Variables|Default|GetHealth) Damage)))
  (if (== _output_get 0)
    (Actor|DestroyActor)
    (else
      (return))))

(fn LeftShotTimer
  (Variables|Default|SetLeftCanFire true))

(fn FireLCanon
  (params (FirePoint :type Arrow%20Component%20Object%20Reference))
  (bind _returnvalue (Transformation|GetWorldRotation FirePoint))
  (if (Variables|Default|GetLeftCanFire)
    (Game|SpawnActorfromClass "/Game/WGF_Content/Blueprint/BP_CanonballProjectile.BP_CanonballProjectile_C" (Math|Transform|MakeTransform (+ (Math|Vector|RotateVector (Variables|Default|GetCannonOffset) _returnvalue) (Transformation|GetWorldLocation FirePoint)) _returnvalue) "Undefined" 0 0)))

(fn FireLeftCannons
  (Utilities|FlowControl|Sequence
    (:then_0
      (CallFunction|FireLCanon (Variables|Default|GetLeftCanon_1)))
    (:then_1
      (CallFunction|FireLCanon (Variables|Default|GetLeftCanon_2)))
    (:then_2
      (CallFunction|FireLCanon (Variables|Default|GetLeftCanon_3)))
    (:then_3
      (Variables|Default|SetLeftCanFire false)
      (Utilities|Time|SetTimerbyFunctionName 0 "LeftShotTimer" (Variables|Default|GetFireRate)))))

(fn FireRightCannons
  (Utilities|FlowControl|Sequence
    (:then_0
      (CallFunction|FireRCanon (Variables|Default|GetRightCanon_1)))
    (:then_1
      (CallFunction|FireRCanon (Variables|Default|GetRightCanon_2)))
    (:then_2
      (CallFunction|FireRCanon (Variables|Default|GetRightCanon_3)))
    (:then_3
      (Variables|Default|SetRightCanFire false)
      (Utilities|Time|SetTimerbyFunctionName 0 "RightShotTimer" (Variables|Default|GetFireRate)))))

(fn RightShotTimer
  (Variables|Default|SetRightCanFire true))

(fn FireRCanon
  (params (FirePoint :type Arrow%20Component%20Object%20Reference))
  (bind _returnvalue (Transformation|GetWorldRotation FirePoint))
  (if (Variables|Default|GetRightCanFire)
    (Game|SpawnActorfromClass "/Game/WGF_Content/Blueprint/BP_CanonballProjectile.BP_CanonballProjectile_C" (Math|Transform|MakeTransform (+ (Math|Vector|RotateVector (Variables|Default|GetCannonOffset) _returnvalue) (Transformation|GetWorldLocation FirePoint)) _returnvalue) "Undefined" 0 0)))

(fn AccelSwitch
  (switch int (Variables|Default|GetAccelarationIndex)
    (:0
      (Variables|Default|SetAccelarationScale 0.0))
    (:1
      (Variables|Default|SetAccelarationScale 0.33))
    (:2
      (Variables|Default|SetAccelarationScale 0.66))
    (:3
      (Variables|Default|SetAccelarationScale 1.0))))

(fn IncreaseIndex
  (if (>= (+ (Variables|Default|GetAccelarationIndex) 1) (Variables|Default|GetMaxAccel))
    (Variables|Default|SetAccelarationIndex (Variables|Default|GetMaxAccel))
    (else
      (Variables|Default|SetAccelarationIndex (+ (Variables|Default|GetAccelarationIndex) 1)))))

(fn DecreaseIndex
  (if (<= (- (Variables|Default|GetAccelarationIndex) 1) (Variables|Default|GetMinAccel))
    (Variables|Default|SetAccelarationIndex 0)
    (else
      (Variables|Default|SetAccelarationIndex (- (Variables|Default|GetAccelarationIndex) 1)))))

(fn Turning
  (params (AxisValue :type Float%20%28single-precision%29))
  (Variables|Default|SetZ-Axis AxisValue)
  (CallFunction|TurnRate)
  (if (<= (+ (.yaw (Transformation|GetWorldRotation (Variables|Default|GetShipMesh))) (+ (Variables|Default|GetTurnRateFl) (Variables|Default|GetZ-Axis))) 0.0)
    (Transformation|SetWorldRotation (Variables|Default|GetShipMesh) (Math|Rotator|MakeRotator 0.0 0.0 (+ (.yaw (Transformation|GetWorldRotation (Variables|Default|GetShipMesh))) (+ (Variables|Default|GetTurnRateFl) (Variables|Default|GetZ-Axis)))) false false)
    (else
      (Transformation|SetWorldRotation (Variables|Default|GetShipMesh) (Math|Rotator|MakeRotator 0.0 0.0 (+ (.yaw (Transformation|GetWorldRotation (Variables|Default|GetShipMesh))) (Variables|Default|GetZ-Axis))) false false))))

(fn TurnRate
  (switch int 0
    (:0
      (Variables|Default|SetTurnRateFl 0.0))
    (:1
      (Variables|Default|SetTurnRateFl -0.25))
    (:2
      (Variables|Default|SetTurnRateFl -0.5))
    (:3
      (Variables|Default|SetTurnRateFl -0.75))))
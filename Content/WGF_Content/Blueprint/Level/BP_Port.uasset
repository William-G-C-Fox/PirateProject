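; BP_Port is a level actor where the player ship banks its treasure and ends the run.
; When a BP_ShipPlayer with at least 50 treasure overlaps its Box, it adds that treasure to the game instance's saved score and writes the save slot.
; A five-second timer then opens MainMenuLevel.
; Each tick, its TextRender rotates to face the player pawn.
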(event OnComponentBeginOverlap(Box)
  (params (OverlappedComponent :type Primitive%20Component%20Object%20Reference) (OtherActor :type Actor%20Object%20Reference) (OtherComp :type Primitive%20Component%20Object%20Reference) (OtherBodyIndex :type Integer) (bFromSweep :type Boolean) (SweepResult :type Hit%20Result%20Structure%20%28by%20ref%29))
  (CallFunction|SaveGame OtherActor))

(event EventBeginPlay)

(event Collision|EventActorBeginOverlap
  (params (OtherActor :type Actor%20Object%20Reference)))

(event EventTick
  (params (DeltaSeconds :type Float%20%28single-precision%29))
  (CallFunction|TextRotateTowardPlayer))

(fn ConstructionScript)

(fn TextRotateTowardPlayer
  (Transformation|SetWorldRotation (Variables|Default|GetTextRender) (Math|Rotator|FindLookatRotation (Transformation|GetWorldLocation (Variables|Default|GetTextRender)) (Transformation|GetActorLocation (Game|Player|GetPlayerPawn 0))) false false))

(fn SaveGame
  (params (Player :type Actor%20Object%20Reference))
  (bind _asbp_ship_player (Utilities|Casting|CastToBP_ShipPlayer Player)
    (:then
      (if (>= (Variables|/Game/WGF_Content/Blueprint/Ship/BP_ShipDefualt.BP_ShipDefualt_C|GetTreasure _asbp_ship_player) 50)
        (bind _asbp_game_instance (Utilities|Casting|CastToBP_GameInstance (Game|GetGameInstance))
          (:then
            (Variables|/Game/WGF_Content/Blueprint/Game/BP_SaveGame.BP_SaveGame_C|SetPlayerScore (Variables|/Game/WGF_Content/Blueprint/Game/BP_GameInstance.BP_GameInstance_C|GetSavedGameData _asbp_game_instance) (+ (Variables|/Game/WGF_Content/Blueprint/Game/BP_SaveGame.BP_SaveGame_C|GetPlayerScore (Variables|/Game/WGF_Content/Blueprint/Game/BP_GameInstance.BP_GameInstance_C|GetSavedGameData _asbp_game_instance)) (Variables|/Game/WGF_Content/Blueprint/Ship/BP_ShipDefualt.BP_ShipDefualt_C|GetTreasure _asbp_ship_player)))
            (SaveGame|SaveGametoSlot (Variables|/Game/WGF_Content/Blueprint/Game/BP_GameInstance.BP_GameInstance_C|GetSavedGameData _asbp_game_instance) (Variables|/Game/WGF_Content/Blueprint/Game/BP_SaveGame.BP_SaveGame_C|GetSaveSlotName (Variables|/Game/WGF_Content/Blueprint/Game/BP_GameInstance.BP_GameInstance_C|GetSavedGameData _asbp_game_instance)))
            (Utilities|Time|SetTimerbyFunctionName 0 "MoveLevel" 5.0))
          (:CastFailed
            (Development|PrintString "failed to cast game instance")
            (return)))
        (else
          (return))))
    (:CastFailed
      (Development|PrintString "cast failed ship")
      (return))))

(fn MoveLevel
  (Game|OpenLevel(byName) "MainMenuLevel"))
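; Player-controllable ship pawn with stepped throttle, steering, port and starboard cannon broadsides, a droppable fire barrel, and health that destroys it at zero.
; Forward/back inputs step an acceleration index that sets the movement scale applied every tick along the actor's right vector.
; Steering yaws the ship mesh, with an opposing offset that slows turning at higher throttle.
; Three-cannon volleys and barrels spawn from scene points, each on separate timer cooldowns sharing FireRate.
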(event EventBeginPlay)

(event Collision|EventActorBeginOverlap
  (params (OtherActor :type Actor%20Object%20Reference)))

(event EventTick
  (params (DeltaSeconds :type Float%20%28single-precision%29))
  (Utilities|FlowControl|Sequence
    (:then_0
      (Pawn|Input|AddMovementInput (Transformation|GetActorRightVector) (Variables|Default|GetAccelarationScale) false))))

(event Input|ActionEvents|InputActionMoveForward
  (params (Key :type Key%20Structure :default "None"))
  (:Pressed
    (CallFunction|IncreaseIndex)
    (CallFunction|AccelSwitch)))

(event Input|ActionEvents|InputActionMoveBack
  (params (Key :type Key%20Structure :default "None"))
  (:Pressed
    (CallFunction|DecreaseIndex)
    (CallFunction|AccelSwitch)))

(event Input|ActionEvents|InputActionFireLeft
  (params (Key :type Key%20Structure :default "None"))
  (:Pressed
    (CallFunction|FireLeftCannons)))

(event Input|ActionEvents|InputActionFireRight
  (params (Key :type Key%20Structure :default "None"))
  (:Pressed
    (CallFunction|FireRightCannons)))

(event Input|ActionEvents|InputActionFireBomb
  (params (Key :type Key%20Structure :default "None"))
  (:Pressed
    (CallFunction|FireBomb (Variables|Default|GetFireBarrel))))

(event Input|AxisEvents|InputAxisMoveRight
  (params (AxisValue :type Float%20%28single-precision%29))
  (CallFunction|Turning AxisValue))

(fn ConstructionScript)

(fn TakeDamage
  (params (Damage :type Integer))
  (bind _output_get (Variables|Default|SetHealth (- (Variables|Default|GetHealth) Damage)))
  (if (<= _output_get 0)
    (Actor|DestroyActor)
    (else
      (return))))

(fn LeftShotTimer
  (Variables|Default|SetLeftCanFire true))

(fn FireLCanon
  (params (FirePoint :type Arrow%20Component%20Object%20Reference))
  (bind _returnvalue (Transformation|GetWorldRotation FirePoint))
  (if (Variables|Default|GetLeftCanFire)
    (Game|SpawnActorfromClass "/Game/WGF_Content/Blueprint/Ship/BP_CanonballProjectile.BP_CanonballProjectile_C" (Math|Transform|MakeTransform (+ (Math|Vector|RotateVector (Variables|Default|GetCannonOffset) _returnvalue) (Transformation|GetWorldLocation FirePoint)) _returnvalue) "Undefined" 0 0)))

(fn FireLeftCannons
  (Utilities|FlowControl|Sequence
    (:then_0
      (CallFunction|FireLCanon (Variables|Default|GetLeftCanon_1)))
    (:then_1
      (CallFunction|FireLCanon (Variables|Default|GetLeftCanon_2)))
    (:then_2
      (CallFunction|FireLCanon (Variables|Default|GetLeftCanon_3)))
    (:then_3
      (Variables|Default|SetLeftCanFire false)
      (Utilities|Time|SetTimerbyFunctionName 0 "LeftShotTimer" (Variables|Default|GetFireRate)))))

(fn FireRightCannons
  (Utilities|FlowControl|Sequence
    (:then_0
      (CallFunction|FireRCanon (Variables|Default|GetRightCanon_1)))
    (:then_1
      (CallFunction|FireRCanon (Variables|Default|GetRightCanon_2)))
    (:then_2
      (CallFunction|FireRCanon (Variables|Default|GetRightCanon_3)))
    (:then_3
      (Variables|Default|SetRightCanFire false)
      (Utilities|Time|SetTimerbyFunctionName 0 "RightShotTimer" (Variables|Default|GetFireRate)))))

(fn RightShotTimer
  (Variables|Default|SetRightCanFire true))

(fn FireRCanon
  (params (FirePoint :type Arrow%20Component%20Object%20Reference))
  (bind _returnvalue (Transformation|GetWorldRotation FirePoint))
  (if (Variables|Default|GetRightCanFire)
    (Game|SpawnActorfromClass "/Game/WGF_Content/Blueprint/Ship/BP_CanonballProjectile.BP_CanonballProjectile_C" (Math|Transform|MakeTransform (+ (Math|Vector|RotateVector (Variables|Default|GetCannonOffset) _returnvalue) (Transformation|GetWorldLocation FirePoint)) _returnvalue) "Undefined" 0 0)))

(fn AccelSwitch
  (switch int (Variables|Default|GetAccelarationIndex)
    (:0
      (Variables|Default|SetAccelarationScale 0.0))
    (:1
      (Variables|Default|SetAccelarationScale 0.33))
    (:2
      (Variables|Default|SetAccelarationScale 0.66))
    (:3
      (Variables|Default|SetAccelarationScale 1.0))))

(fn IncreaseIndex
  (if (>= (+ (Variables|Default|GetAccelarationIndex) 1) (Variables|Default|GetMaxAccel))
    (Variables|Default|SetAccelarationIndex (Variables|Default|GetMaxAccel))
    (else
      (Variables|Default|SetAccelarationIndex (+ (Variables|Default|GetAccelarationIndex) 1)))))

(fn DecreaseIndex
  (if (<= (- (Variables|Default|GetAccelarationIndex) 1) (Variables|Default|GetMinAccel))
    (Variables|Default|SetAccelarationIndex 0)
    (else
      (Variables|Default|SetAccelarationIndex (- (Variables|Default|GetAccelarationIndex) 1)))))

(fn Turning
  (params (AxisValue :type Float%20%28single-precision%29))
  (bind _output_get (Variables|Default|SetZ-Axis AxisValue))
  (if (== _output_get 0.0)
    (return)
    (else
      (CallFunction|TurnRate)
      (Transformation|SetWorldRotation (Variables|Default|GetShipMesh) (Math|Rotator|MakeRotator 0.0 0.0 (+ (.yaw (Transformation|GetWorldRotation (Variables|Default|GetShipMesh))) (+ (Variables|Default|GetTurnRateFl) (Variables|Default|GetZ-Axis)))) false false))))

(fn TurnRate
  (if (== (Variables|Default|GetZ-Axis) 0.0)
    (Variables|Default|SetTurnRateFl 0.0)
    (elif (== (Variables|Default|GetZ-Axis) 1.0)
      (switch int (Variables|Default|GetAccelarationIndex)
        (:0
          (Variables|Default|SetTurnRateFl 0.0))
        (:1
          (Variables|Default|SetTurnRateFl -0.15))
        (:2
          (Variables|Default|SetTurnRateFl -0.35))
        (:3
          (Variables|Default|SetTurnRateFl -0.55)))
      (elif (== (Variables|Default|GetZ-Axis) -1.0)
        (switch int (Variables|Default|GetAccelarationIndex)
          (:0
            (Variables|Default|SetTurnRateFl 0.0))
          (:1
            (Variables|Default|SetTurnRateFl 0.15))
          (:2
            (Variables|Default|SetTurnRateFl 0.35))
          (:3
            (Variables|Default|SetTurnRateFl 0.55)))))))

(fn FireBomb
  (params (FireBomb :type Arrow%20Component%20Object%20Reference))
  (bind _returnvalue (Transformation|GetWorldRotation FireBomb))
  (if (Variables|Default|GetFireBombRate)
    (Game|SpawnActorfromClass "/Game/WGF_Content/Blueprint/Ship/BP_FireBarrel.BP_FireBarrel_C" (Math|Transform|MakeTransform (+ (Math|Vector|RotateVector (Variables|Default|GetFireBarrelOffset) _returnvalue) (Transformation|GetWorldLocation FireBomb)) _returnvalue) "Undefined" 0 0)
    (Variables|Default|SetFireBombRate false)
    (Utilities|Time|SetTimerbyFunctionName 0 "FireBombTimer" (Variables|Default|GetFireRate))
    (else
      (return))))

(fn FireBombTimer
  (Variables|Default|SetFireBombRate true))
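; Player-controlled ship that sails constantly along its forward vector, scaled by an acceleration value that forward/back presses step through indexed settings.
; Input also drives turning, port and starboard cannons, barrel bombs and spring-arm yaw; camera pitch is left unwired.
; Collected treasure raises notoriety only when the total lands exactly 100 above the last checkpoint.
; It creates the HUD in the gameplay level and can swap it for the lose screen.
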(event EventBeginPlay
  (|CallParentFunction)
  (CallFunction|MainMenuHUd))

(event Collision|EventActorBeginOverlap
  (params (OtherActor :type Actor%20Object%20Reference))
  (|CallParentFunction OtherActor) ; This node is disabled and will not be called.\nDrag off pins to build functionality.
)

(event EventTick
  (params (DeltaSeconds :type Float%20%28single-precision%29))
  ;[1 1 1] Movement for the player ship
  (|CallParentFunction DeltaSeconds)
  (Pawn|Input|AddMovementInput (Transformation|GetActorForwardVector) (Variables|Default|GetAccelarationScale) false))

(event Input|ActionEvents|InputActionMoveForward
  (params (Key :type Key%20Structure))
  ;[1 1 1] All the user input
  (:Pressed
    (CallFunction|IncreaseIndex)
    (CallFunction|AccelSwitch)))

(event Input|ActionEvents|InputActionMoveBack
  (params (Key :type Key%20Structure))
  ;[1 1 1] All the user input
  (:Pressed
    (CallFunction|DecreaseIndex)
    (CallFunction|AccelSwitch)))

(event Input|ActionEvents|InputActionFireLeft
  (params (Key :type Key%20Structure))
  ;[1 1 1] All the user input
  (:Pressed
    (CallFunction|FireLeftCannons)))

(event Input|ActionEvents|InputActionFireRight
  (params (Key :type Key%20Structure))
  ;[1 1 1] All the user input
  (:Pressed
    (CallFunction|FireRightCannons)))

(event Input|ActionEvents|InputActionFireBomb
  (params (Key :type Key%20Structure))
  ;[1 1 1] All the user input
  (:Pressed
    (CallFunction|FireBomb (Variables|Default|GetFireBarrel))))

(event Input|AxisEvents|InputAxisMoveCameraRight
  (params (AxisValue :type Float%20%28single-precision%29))
  ;[1 1 1] All the user input
  (CallFunction|TurnCameraLR AxisValue))

(event Input|AxisEvents|InputAxisMoveRight
  (params (AxisValue :type Float%20%28single-precision%29))
  ;[1 1 1] All the user input
  (CallFunction|Turning AxisValue))

(event Input|AxisEvents|InputAxisMoveCameraUD
  (params (AxisValue :type Float%20%28single-precision%29))
  ;[1 1 1] All the user input
)

(fn ConstructionScript
  (|CallParentFunction))

(fn TurnCameraLR
  (params (Axis :type Float%20%28single-precision%29))
  (Variables|Default|SetCameraZAxis Axis)
  (Transformation|SetWorldRotation (Variables|Default|GetSpringArm) (Math|Rotator|MakeRotator 0.0 0.0 (+ (.yaw (Transformation|GetWorldRotation (Variables|Default|GetSpringArm))) (Variables|Default|GetCameraZAxis))) false false))

(fn TurnCameraUD
  (params (Axis :type Float%20%28single-precision%29))
  (Variables|Default|SetCameraYAxis Axis)
  (Transformation|SetWorldRotation (Variables|Default|GetCamera) (Math|Rotator|MakeRotator 0.0 (Math|Float|Clamp(Float) 0.0 (+ (.pitch (Transformation|GetWorldRotation (Variables|Default|GetCamera))) (Variables|Default|GetCameraYAxis)) 45.0) 0.0) false false))

(fn IncreaseNotority
  (if (== (Variables|Default|GetTreasure) (+ (Variables|Default|GetTreasureCheck) 100))
    (Variables|Default|SetNotority (+ (Variables|Default|GetNotority) 1))
    (Variables|Default|SetTreasureCheck (Variables|Default|GetTreasure))
    (if (== (Variables|Default|GetNotority) 5)
      (Variables|Default|SetNotority 5)
      (else
        (return)))
    (else
      (return))))

(fn IncreaseTreasure
  (params (TreasureCollected :type Integer))
  (Variables|Default|SetTreasure (+ TreasureCollected (Variables|Default|GetTreasure)))
  (CallFunction|IncreaseNotority))

(fn RemoveHud
  (Widget|RemovefromParent (Variables|Default|GetHUD))
  (bind _returnvalue (UserInterface|CreateWidget "/Game/WGF_Content/UI/WB_Lose.WB_Lose_C"))
  (UserInterface|Viewport|AddtoViewport _returnvalue 0))

(fn MainMenuHUd
  (bind _returnvalue (Game|GetCurrentLevelName true))
  (switch string _returnvalue
    (:MainMenu
      (return))
    (:Level
      (bind _returnvalue_2 (UserInterface|CreateWidget "/Game/WGF_Content/UI/WB_HUD.WB_HUD_C"))
      (bind _output_get (Variables|Default|SetHUD _returnvalue_2))
      (UserInterface|Viewport|AddtoViewport _output_get 0))))
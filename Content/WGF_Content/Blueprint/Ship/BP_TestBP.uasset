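; Test ship Blueprint with an AITurn function that snaps its Ship component to face a given target point.
; AITurn takes pitch and yaw from a look-at rotation, zeroes roll, and sets the world rotation directly without interpolation or sweep.
; It also prints debug strings, including the computed rotation.
; The event graph and construction script are empty, and nothing in this Blueprint calls AITurn.
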(event EventBeginPlay)

(event Collision|EventActorBeginOverlap
  (params (OtherActor :type Actor%20Object%20Reference)))

(event EventTick
  (params (DeltaSeconds :type Float%20%28single-precision%29)))

(fn ConstructionScript)

(fn AITurn
  (params (Target :type Vector))
  (bind _ship (Variables|Default|GetShip))
  (bind _returnvalue (Transformation|GetWorldLocation _ship))
  (bind _returnvalue_2 (Math|Rotator|FindLookatRotation _returnvalue Target))
  (bind _returnvalue_3 (Math|Rotator|MakeRotator 0.0 (.pitch _returnvalue_2) (.yaw _returnvalue_2)))
  (Development|PrintString (Utilities|String|ToString(Vector) "0, 0, 0"))
  (Development|PrintString (Utilities|String|ToString(Vector) "0, 0, 0"))
  (Development|PrintString (Utilities|String|ToString(Rotator) _returnvalue_3))
  (Transformation|SetWorldRotation (Variables|Default|GetShip) _returnvalue_3 false false))